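; Actor that switches a rug material on its Plane mesh and shows a color-change UI while something overlaps its Box.
; Box begin overlap adds a Colorchange widget and enables Game and UI input with a visible cursor.
; End overlap removes all widgets and restores game-only input, but leaves the cursor visible.
; Pink, purple and yellow events each apply a different M_Master_Rug instance to the Plane.
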(event OnComponentBeginOverlap(Box)
  (params (OverlappedComponent :type Primitive%20Component%20Object%20Reference) (OtherActor :type Actor%20Object%20Reference) (OtherComp :type Primitive%20Component%20Object%20Reference) (OtherBodyIndex :type Integer) (bFromSweep :type Boolean) (SweepResult :type Hit%20Result%20Structure%20%28by%20ref%29))
  (bind _returnvalue (Game|GetPlayerController 0))
  (bind _returnvalue_2 (UserInterface|CreateWidget "/Game/Material_Switching/colorchange.colorchange_C"))
  (UserInterface|Viewport|AddtoViewport _returnvalue_2 0)
  (Input|SetInputModeGameandUI _returnvalue 0 "DoNotLock" true)
  (Variables|/Script/Engine.PlayerController|SetbShowMouseCursor _returnvalue true))

(event OnComponentEndOverlap(Box)
  (params (OverlappedComponent :type Primitive%20Component%20Object%20Reference) (OtherActor :type Actor%20Object%20Reference) (OtherComp :type Primitive%20Component%20Object%20Reference) (OtherBodyIndex :type Integer))
  (bind _returnvalue (Game|GetPlayerController 0))
  (Viewport|RemoveAllWidgets)
  (Input|SetInputModeGameOnly _returnvalue)
  (Variables|/Script/Engine.PlayerController|SetbShowMouseCursor _returnvalue true))

(event Custom|Is%20Pink?
  (Rendering|Material|SetMaterial (Variables|Default|GetPlane) 0 "/Game/Bedroom/Rug/mesh/M_Master_Rug_Inst1.M_Master_Rug_Inst1"))

(event Custom|Is%20Purple?
  (Rendering|Material|SetMaterial (Variables|Default|GetPlane) 0 "/Game/Bedroom/Rug/mesh/M_Master_Rug_Inst2.M_Master_Rug_Inst2"))

(event Custom|Is%20Yellow?
  (Rendering|Material|SetMaterial (Variables|Default|GetPlane) 0 "/Game/Bedroom/Rug/mesh/M_Master_Rug_Inst.M_Master_Rug_Inst"))

(fn ConstructionScript)