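; Bathroom sink Blueprint that lets the player switch the small sink's material between white, grey and black marble.
; Overlapping the sink's collision opens a selection widget, switches input to game and UI, and shows the cursor.
; Three events, one per marble, set the mesh's first material slot; their caller is outside this graph.
; Ending the overlap removes all widgets and restores game-only input, but leaves the cursor flag on.
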(event OnComponentBeginOverlap(SmallSinkCollision)
  (params (OverlappedComponent :type Primitive%20Component%20Object%20Reference) (OtherActor :type Actor%20Object%20Reference) (OtherComp :type Primitive%20Component%20Object%20Reference) (OtherBodyIndex :type Integer) (bFromSweep :type Boolean) (SweepResult :type Hit%20Result%20Structure%20%28by%20ref%29))
  (bind _returnvalue (Game|GetPlayerController 0))
  (bind _returnvalue_2 (UserInterface|CreateWidget "/Game/Material_Switching/Mat_2BathSinkChange_sink2.Mat_2BathSinkChange_sink2_C"))
  (UserInterface|Viewport|AddtoViewport _returnvalue_2 0)
  (Input|SetInputModeGameandUI _returnvalue 0 "DoNotLock" true)
  (Variables|/Script/Engine.PlayerController|SetbShowMouseCursor _returnvalue true))

(event OnComponentEndOverlap(SmallSinkCollision)
  (params (OverlappedComponent :type Primitive%20Component%20Object%20Reference) (OtherActor :type Actor%20Object%20Reference) (OtherComp :type Primitive%20Component%20Object%20Reference) (OtherBodyIndex :type Integer))
  (bind _returnvalue (Game|GetPlayerController 0))
  (Viewport|RemoveAllWidgets)
  (Input|SetInputModeGameOnly _returnvalue)
  (Variables|/Script/Engine.PlayerController|SetbShowMouseCursor _returnvalue true))

(event Custom|Sink2_iswhite
  (Rendering|Material|SetMaterial (Variables|Default|GetSinksmallMatChange) 0 "/Game/Material_Switching/M_IsWhiteMarble.M_IsWhiteMarble"))

(event Custom|Sink2_isGrey
  (Rendering|Material|SetMaterial (Variables|Default|GetSinksmallMatChange) 0 "/Game/Material_Switching/M_IsGreyMarble.M_IsGreyMarble"))

(event Custom|Sink2_isblack
  (Rendering|Material|SetMaterial (Variables|Default|GetSinksmallMatChange) 0 "/Game/Material_Switching/M_IsBlackMarble.M_IsBlackMarble"))

(fn ConstructionScript)