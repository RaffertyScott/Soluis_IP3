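; BP_BathSinkChange is an actor that switches a bathroom sink's wood finish between light, medium and dark materials.
; Three custom events each set one material slot on the SinkColourchange component.
; Overlapping Sink_collision opens the Mat_Change_sink widget with game-and-UI input and a visible cursor.
; Ending overlap removes all widgets and restores game-only input, but leaves the cursor visible.
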(event OnComponentBeginOverlap(sink_collision)
  (params (OverlappedComponent :type Primitive%20Component%20Object%20Reference) (OtherActor :type Actor%20Object%20Reference) (OtherComp :type Primitive%20Component%20Object%20Reference) (OtherBodyIndex :type Integer) (bFromSweep :type Boolean) (SweepResult :type Hit%20Result%20Structure%20%28by%20ref%29))
  (bind _returnvalue (Game|GetPlayerController 0))
  (bind _returnvalue_2 (UserInterface|CreateWidget "/Game/Material_Switching/Mat_Change_sink.Mat_Change_sink_C"))
  (UserInterface|Viewport|AddtoViewport _returnvalue_2 0)
  (Input|SetInputModeGameandUI _returnvalue 0 "DoNotLock" true)
  (Variables|/Script/Engine.PlayerController|SetbShowMouseCursor _returnvalue true))

(event OnComponentEndOverlap(sink_collision)
  (params (OverlappedComponent :type Primitive%20Component%20Object%20Reference) (OtherActor :type Actor%20Object%20Reference) (OtherComp :type Primitive%20Component%20Object%20Reference) (OtherBodyIndex :type Integer))
  (bind _returnvalue (Game|GetPlayerController 0))
  (Viewport|RemoveAllWidgets)
  (Input|SetInputModeGameOnly _returnvalue)
  (Variables|/Script/Engine.PlayerController|SetbShowMouseCursor _returnvalue true))

(event Custom|isLightWood?
  (Rendering|Material|SetMaterial (Variables|Default|Getsink_colourchange) 2 "/Game/Material_Switching/M_MatWood_L.M_MatWood_L"))

(event Custom|isMediumWood?
  (Rendering|Material|SetMaterial (Variables|Default|Getsink_colourchange) 2 "/Game/Material_Switching/M_MatWood_M.M_MatWood_M"))

(event Custom|isDarkWood?
  (Rendering|Material|SetMaterial (Variables|Default|Getsink_colourchange) 2 "/Game/Material_Switching/M_MatWood_D.M_MatWood_D"))

(fn ConstructionScript)