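; Chair actor Blueprint that lets its material be switched between white, grey and blue variants.
; Overlapping the chair's collision box opens the Match_Change_Chair widget with Game and UI input and a visible cursor.
; Three custom events each set one material on ChairCollision's first slot.
; Ending the overlap removes all widgets and restores game-only input, though the cursor flag stays on.
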(event OnComponentBeginOverlap(Chair_collision_box)
  (params (OverlappedComponent :type Primitive%20Component%20Object%20Reference) (OtherActor :type Actor%20Object%20Reference) (OtherComp :type Primitive%20Component%20Object%20Reference) (OtherBodyIndex :type Integer) (bFromSweep :type Boolean) (SweepResult :type Hit%20Result%20Structure%20%28by%20ref%29))
  (bind _returnvalue (Game|GetPlayerController 0))
  (bind _returnvalue_2 (UserInterface|CreateWidget "/Game/Material_Switching/Match_Change_Chair.Match_Change_Chair_C"))
  (UserInterface|Viewport|AddtoViewport _returnvalue_2 0)
  (Input|SetInputModeGameandUI _returnvalue 0 "DoNotLock" true)
  (Variables|/Script/Engine.PlayerController|SetbShowMouseCursor _returnvalue true))

(event OnComponentEndOverlap(Chair_collision_box)
  (params (OverlappedComponent :type Primitive%20Component%20Object%20Reference) (OtherActor :type Actor%20Object%20Reference) (OtherComp :type Primitive%20Component%20Object%20Reference) (OtherBodyIndex :type Integer))
  (bind _returnvalue (Game|GetPlayerController 0))
  (Viewport|RemoveAllWidgets)
  (Input|SetInputModeGameOnly _returnvalue)
  (Variables|/Script/Engine.PlayerController|SetbShowMouseCursor _returnvalue true))

(event Custom|isWhite?
  (Rendering|Material|SetMaterial (Variables|Default|GetChair_collision) 0 "/Game/Material_Switching/M_ChairIs_White.M_ChairIs_White"))

(event Custom|isGrey?
  (Rendering|Material|SetMaterial (Variables|Default|GetChair_collision) 0 "/Game/Material_Switching/M_ChairIsGrey.M_ChairIsGrey"))

(event Custom|isBlue?
  (Rendering|Material|SetMaterial (Variables|Default|GetChair_collision) 0 "/Game/Material_Switching/M_ChairIsBlue.M_ChairIsBlue"))

(fn ConstructionScript)