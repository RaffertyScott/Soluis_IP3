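; Blueprint for a kitchen floor whose tile material the player can switch between grey, brown and black.
; Entering its collision box opens the Colorchange_kitchen_floor widget with Game and UI input and a visible cursor.
; Three custom events each set a tile material on the floor mesh's first slot.
; Leaving the box removes all widgets and restores game-only input, but keeps the cursor flag on.
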(event OnComponentBeginOverlap(Box_collision_kit_floor)
  (params (OverlappedComponent :type Primitive%20Component%20Object%20Reference) (OtherActor :type Actor%20Object%20Reference) (OtherComp :type Primitive%20Component%20Object%20Reference) (OtherBodyIndex :type Integer) (bFromSweep :type Boolean) (SweepResult :type Hit%20Result%20Structure%20%28by%20ref%29))
  (bind _returnvalue (Game|GetPlayerController 0))
  (bind _returnvalue_2 (UserInterface|CreateWidget "/Game/Material_Switching/colorchange_kitchen_floor.colorchange_kitchen_floor_C"))
  (UserInterface|Viewport|AddtoViewport _returnvalue_2 0)
  (Input|SetInputModeGameandUI _returnvalue 0 "DoNotLock" true)
  (Variables|/Script/Engine.PlayerController|SetbShowMouseCursor _returnvalue true))

(event OnComponentEndOverlap(Box_collision_kit_floor)
  (params (OverlappedComponent :type Primitive%20Component%20Object%20Reference) (OtherActor :type Actor%20Object%20Reference) (OtherComp :type Primitive%20Component%20Object%20Reference) (OtherBodyIndex :type Integer))
  (bind _returnvalue (Game|GetPlayerController 0))
  (Viewport|RemoveAllWidgets)
  (Input|SetInputModeGameOnly _returnvalue)
  (Variables|/Script/Engine.PlayerController|SetbShowMouseCursor _returnvalue true))

(event Custom|isGrey?
  (Rendering|Material|SetMaterial (Variables|Default|GetR_Changable_Kit_floor) 0 "/Game/Material_Switching/Grey_Tiles_2x2_M_00_inst1.Grey_Tiles_2x2_M_00_inst1"))

(event Custom|isBrown?
  (Rendering|Material|SetMaterial (Variables|Default|GetR_Changable_Kit_floor) 0 "/Game/Material_Switching/Grey_Tiles_2x2_M_00_inst1_Inst.Grey_Tiles_2x2_M_00_inst1_Inst"))

(event Custom|isBlack?
  (Rendering|Material|SetMaterial (Variables|Default|GetR_Changable_Kit_floor) 0 "/Game/Material_Switching/Black_Tiles_2x2_M_00_inst1.Black_Tiles_2x2_M_00_inst1"))

(fn ConstructionScript)