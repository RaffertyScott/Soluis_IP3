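; Blueprint for switching a living room wall material between red, grey and blue through an on-screen menu.
; Entering the wall collision box creates the Mat_change_Wall widget and enables Game and UI input with a mouse cursor.
; Three color events each set material slot 1 on the living room mesh.
; Leaving the box removes all widgets and restores game-only input, though the cursor stays visible.
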(event OnComponentBeginOverlap(Wall_Box_Collision)
  (params (OverlappedComponent :type Primitive%20Component%20Object%20Reference) (OtherActor :type Actor%20Object%20Reference) (OtherComp :type Primitive%20Component%20Object%20Reference) (OtherBodyIndex :type Integer) (bFromSweep :type Boolean) (SweepResult :type Hit%20Result%20Structure%20%28by%20ref%29))
  (bind _returnvalue (Game|GetPlayerController 0))
  (bind _returnvalue_2 (UserInterface|CreateWidget "/Game/Material_Switching/Mat_change_Wall.Mat_change_Wall_C"))
  (UserInterface|Viewport|AddtoViewport _returnvalue_2 0)
  (Input|SetInputModeGameandUI _returnvalue 0 "DoNotLock" true)
  (Variables|/Script/Engine.PlayerController|SetbShowMouseCursor _returnvalue true))

(event OnComponentEndOverlap(Wall_Box_Collision)
  (params (OverlappedComponent :type Primitive%20Component%20Object%20Reference) (OtherActor :type Actor%20Object%20Reference) (OtherComp :type Primitive%20Component%20Object%20Reference) (OtherBodyIndex :type Integer))
  (bind _returnvalue (Game|GetPlayerController 0))
  (Viewport|RemoveAllWidgets)
  (Input|SetInputModeGameOnly _returnvalue)
  (Variables|/Script/Engine.PlayerController|SetbShowMouseCursor _returnvalue true))

(event Custom|IsRed?
  (Rendering|Material|SetMaterial (Variables|Default|Getliving_room_update_Mesh2) 1 "/Game/Material_Switching/1.1"))

(event Custom|IsGrey
  (Rendering|Material|SetMaterial (Variables|Default|Getliving_room_update_Mesh2) 1 "/Game/Material_Switching/2.2"))

(event Custom|IsBlue
  (Rendering|Material|SetMaterial (Variables|Default|Getliving_room_update_Mesh2) 1 "/Game/Material_Switching/3.3"))

(fn ConstructionScript)